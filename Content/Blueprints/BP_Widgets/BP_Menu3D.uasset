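; BP_Menu3D is a world-placed menu actor that shows a BPW_Menu3D widget and links to other menus for navigation.
; On BeginPlay it binds to the widget's transition event, which passes an index into the LinkedMenu array.
; A valid index moves collision from this menu to the target and blends the player's view target to it with an eased camera transition.
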(event Custom|TransitionTo
  (params (NewMenu :type BP%20Menu%203D%20Object%20Reference))
  (Collision|SetActorEnableCollision false)
  (Collision|SetActorEnableCollision NewMenu true)
  (Game|Player|SetViewTargetwithBlend (Game|GetPlayerController 0) NewMenu 1.5 "VTBlend_EaseInOut" 2.0 false))

(event Custom|OnTransitionBetweenMenus
  (params (InstructionsIndex :type Integer))
  (bind _linkedmenu (Variables|Default|GetLinkedMenu))
  (if (Utilities|Array|IsValidIndex _linkedmenu InstructionsIndex)
    (CallFunction|Transitionto (Utilities|Array|Get(acopy) _linkedmenu InstructionsIndex))))

(event EventBeginPlay
  (bind _asbpw_menu_3d (Utilities|Casting|CastToBPW_Menu3D (UserInterface|GetUserWidgetObject (Variables|Default|GetWidget))))
  (EventDispatchers|BindEventtoTransitiontoLinkedMenu _asbpw_menu_3d (delegate Custom|OnTransitionBetweenMenus)))

(fn ConstructionScript)