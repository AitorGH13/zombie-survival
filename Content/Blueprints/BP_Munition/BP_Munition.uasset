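; BP_Munition is an ammo pickup with a mesh and spotlight that reports to BP_Guide_GameMode.
; On player overlap it calls MunitionCollected, plays an equip sound, destroys its components and increments CollectedMunitionCount.
; Tick caches the game mode and compares that count to Wave: below it, a DoOnce runs the same destroy-and-increment chain; otherwise the DoOnce resets.
; InitMunition is empty, and a Teleport node is unconnected.
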(event Collision|EventActorBeginOverlap
  (params (OtherActor :type Actor%20Object%20Reference))
  ;[1 1 1] Eliminar munición si colsiona con el jugador
  (if (== OtherActor (Game|GetPlayerCharacter 0))
    (Default|MunitionCollected (Variables|Default|GetMy%20Guide%20GameMode))
    (Audio|PlaySound2D "/Game/Blueprints/BP_Munition/Sounds/ItemEquip.ItemEquip" 1.0 1.0 0.0 0 0)
    (Components|DestroyComponent (Variables|Default|GetDefaultSceneRoot))
    (bind _result (Math|Integer|IncrementInt (Variables|/Game/Blueprints/BP_Guide/BP_Guide_GameMode.BP_Guide_GameMode_C|GetCollectedMunitionCount (stale EventTick _output_get)))
      (:%20%20
        (Variables|/Game/Blueprints/BP_Guide/BP_Guide_GameMode.BP_Guide_GameMode_C|SetCollectedMunitionCount (stale EventTick _output_get) _result)))))

(event EventTick
  (params (DeltaSeconds :type Float%20%28single-precision%29))
  ;[1 1 1] Spawnear municion solo en oleada 3
  (bind _asbp_guide_game_mode (Utilities|Casting|CastToBP_Guide_GameMode (Game|GetGameMode)))
  (bind _output_get (Variables|Default|SetMy%20Guide%20GameMode _asbp_guide_game_mode))
  (if (>= (Variables|/Game/Blueprints/BP_Guide/BP_Guide_GameMode.BP_Guide_GameMode_C|GetCollectedMunitionCount _output_get) (Variables|/Game/Blueprints/BP_Guide/BP_Guide_GameMode.BP_Guide_GameMode_C|GetWave _output_get))
    (goto _label Reset)
    (else
      (Utilities|FlowControl|DoOnce false :!label _label
        (:Completed
          ;[1 1 1] Eliminar munición si colsiona con el jugador
          (Components|DestroyComponent (Variables|Default|GetDefaultSceneRoot))
          (bind _result (Math|Integer|IncrementInt (Variables|/Game/Blueprints/BP_Guide/BP_Guide_GameMode.BP_Guide_GameMode_C|GetCollectedMunitionCount _output_get))
            (:%20%20
              (Variables|/Game/Blueprints/BP_Guide/BP_Guide_GameMode.BP_Guide_GameMode_C|SetCollectedMunitionCount _output_get _result))))))))

(fn ConstructionScript)

(fn InitMunition)