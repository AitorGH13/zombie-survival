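; BP_SpeedMunition is a speed munition pickup actor that the player collects by overlapping it.
; On BeginPlay it caches BP_Guide_GameMode and, after a one-minute delay, InitSpeedMun teleports it to a hardcoded world location.
; Player overlap calls SpeedMunitionCollected on the game mode, then destroys the root and mesh components rather than the actor itself.
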(event EventBeginPlay
  ;[1 1 1] Crear municion
  (bind _asbp_guide_game_mode (Utilities|Casting|CastToBP_Guide_GameMode (Game|GetGameMode)))
  (Variables|Default|SetMy%20Guide%20GameMode _asbp_guide_game_mode)
  (Utilities|FlowControl|Delay 6e+01)
  (CallFunction|InitSpeedMun))

(event Collision|EventActorBeginOverlap
  (params (OtherActor :type Actor%20Object%20Reference))
  ;[1 1 1] Spawnear Municion
  (if (== OtherActor (Game|GetPlayerCharacter 0))
    (Default|SpeedMunitionCollected (Variables|Default|GetMy%20Guide%20GameMode))
    (Components|DestroyComponent (Variables|Default|GetDefaultSceneRoot))))

(fn ConstructionScript)

(fn InitSpeedMun
  (Transformation|Teleport "-3480.000000,-40.000000,310.000000" "0, 0, 0"))