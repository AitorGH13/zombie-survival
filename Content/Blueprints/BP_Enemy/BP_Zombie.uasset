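; BP_Zombie is an enemy character that chases the player, plays random ambient groans and attacks in melee.
; Pawn sensing drives AIMoveTo into an attack montage, whose completion calls the game mode's Hit.
; An overlap sphere latches PlayerClose, letting Tick path toward an unseen player.
; Tick also sets later-wave walk speed, yaws the health bar toward the player, and handles death, incrementing the player's kill count.
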(event OnComponentBeginOverlap(Sphere)
  (params (OverlappedComponent :type Primitive%20Component%20Object%20Reference) (OtherActor :type Actor%20Object%20Reference) (OtherComp :type Primitive%20Component%20Object%20Reference) (OtherBodyIndex :type Integer) (bFromSweep :type Boolean) (SweepResult :type Hit%20Result%20Structure%20%28by%20ref%29))
  ;[1 1 1] Detectar jugador mediante colisión
  (if (Actor|ActorHasTag OtherActor "Jugador")
    (Variables|Default|SetPlayerClose true)))

(event OnSeePawn(PawnSensing)
  (params (Pawn :type Pawn%20Object%20Reference))
  ;[1 1 1] Movimiento enemigo (cuando nos ve)
  (Variables|Default|SetSeesPlayer true)
  (bind _asfirst_person_character (Utilities|Casting|CastToFirstPersonCharacter Pawn))
  (AI|AIMoveTo self "0, 0, 0" _asfirst_person_character 15.0 false
    (:OnSuccess
      (Variables|Default|SetSeesPlayer false)
      (if (not (Class|AnimInstance|IsAnyMontagePlaying (Components|SkeletalMesh|GetAnimInstance (Variables|Character|GetMesh))))
        ;[1 1 1] Enemigo ataque
        (Animation|Montage|PlayMontage (Variables|Character|GetMesh) "/Game/Blueprints/BP_Enemy/AM_ZombieAttack.AM_ZombieAttack"
          (:then
            (Audio|PlaySoundatLocation "/Game/Blueprints/BP_Enemy/Sounds/AtqueZombie.AtqueZombie" "0, 0, 0" "0, 0, 0" 1.0 1.0 0.0 0 0 0 0))
          (:OnCompleted
            (Default|Hit (Variables|Default|GetMy%20Guide%20Game%20Mode))))))))

(event Custom|IncrementarZombieMuertos
  ;[1 1 1] IncrementarZombieMuertos
  (bind _asfirst_person_character (Utilities|Casting|CastToFirstPersonCharacter (Game|GetPlayerCharacter 0)))
  (Variables|/Game/Blueprints/BP_FirstPerson/FirstPersonCharacter.FirstPersonCharacter_C|SetDeadZombieNumber _asfirst_person_character (+ (Variables|/Game/Blueprints/BP_FirstPerson/FirstPersonCharacter.FirstPersonCharacter_C|GetDeadZombieNumber _asfirst_person_character) 1)))

(event EventBeginPlay
  ;[1 1 1] Ruido zombie
  (Utilities|FlowControl|Sequence
    (:then_0
      (bind _asbp_guide_game_mode (Utilities|Casting|CastToBP_Guide_GameMode (Game|GetGameMode)))
      (Variables|Default|SetMy%20Guide%20Game%20Mode _asbp_guide_game_mode))
    (:then_1
      (Utilities|FlowControl|Delay (Math|Conversions|ToFloat(Integer) (Math|Random|RandomIntegerinRange 5 30)) :!label _label)
      (Audio|PlaySoundatLocation "/Game/Blueprints/BP_Enemy/Sounds/SonidoStandarZombie.SonidoStandarZombie" (Transformation|GetActorLocation) "0, 0, 0" 1.0 1.0 0.0 0 0 0 0)
      (goto _label))))

(event EventTick
  (params (DeltaSeconds :type Float%20%28single-precision%29))
  (Utilities|FlowControl|Sequence
    (:then_0
      ;[1 1 1] Aumentar ligeramnete velocidad cuando oleada >= 4
      (bind _asbp_guide_game_mode (Utilities|Casting|CastToBP_Guide_GameMode (Game|GetGameMode)))
      (if (>= (Variables|/Game/Blueprints/BP_Guide/BP_Guide_GameMode.BP_Guide_GameMode_C|GetWave _asbp_guide_game_mode) 4)
        (Utilities|FlowControl|Delay 1.0)
        (Variables|/Script/Engine.CharacterMovementComponent|SetMaxWalkSpeed (Variables|Character|GetCharacterMovement) 1.2e+02)))
    (:then_1
      (if (<= (Variables|Default|GetEnemyHealth) 0.0)
        ;[1 1 1] Muerte enemigo
        (Physics|SetSimulatePhysics (Variables|Character|GetMesh) true)
        (CallFunction|IncrementarZombieMuertos)
        (Actor|DestroyActor)
        (Audio|PlaySoundatLocation "/Game/Blueprints/BP_Enemy/Sounds/Death_Zombie.Death_Zombie" (Transformation|GetActorLocation) "0, 0, 0" 1.0 1.0 0.0 0 0 0 0)
        (else
          ;[1 1 1] Barra de salud de enemigo
          (bind _asbpw_enemy_health (Utilities|Casting|CastToBPW_EnemyHealth (UserInterface|GetUserWidgetObject (Variables|Components|GetWidget))))
          (Progress|SetPercent (Variables|/Game/Blueprints/BP_Widgets/Widgets/BPW_EnemyHealth.BPW_EnemyHealth_C|GetProgressBar_EnemieHealth _asbpw_enemy_health) (/ (Variables|Default|GetEnemyHealth) 1e+02))
          (Transformation|SetWorldRotation (Variables|Components|GetWidget) (Math|Rotator|MakeRotator 0.0 0.0 (.Yaw (Math|Rotator|BreakRotator (Math|Rotator|FindLookatRotation (Transformation|GetWorldLocation (Variables|Components|GetWidget)) (Transformation|GetActorLocation (Game|GetPlayerCharacter 0)))))) false false))))
    (:then_2
      ;[1 1 1] Ir hacia la ubicacion del jugador si estoy cerca y no me ve
      (if (Variables|Default|GetPlayerClose)
        (if (not (Variables|Default|GetSeesPlayer))
          (AI|Navigation|SimpleMovetoLocation (Pawn|GetController) (Transformation|GetActorLocation (.AsFirst%20Person%20Character (Utilities|Casting|CastToFirstPersonCharacter (Game|GetPlayerCharacter 0))))))))))

(fn ConstructionScript)