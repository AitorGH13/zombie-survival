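; Game mode for a first-person shooter that holds health, munition, wave and time, and decides when the player wins or loses.
; StartGame resets these values on BeginPlay or restart and starts a looping one-second Clock timer.
; Clock counts time and checks health and the character's kill count, pausing into a game-over or win screen with sound.
; Helper functions apply shots, hits and pickups to the state.
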(event Custom|RestartGame
  (Utilities|StartGame))

(event Custom|Clock
  (bind _returnvalue (Game|GetPlayerController 0))
  (bind _returnvalue_2 (Game|GetPlayerController 0))
  (Variables|Default|SetTime (+ (Variables|Default|GetTime) 1))
  (if (<= (Variables|Default|GetHealth) 0)
    ;[1 1 1] Jugador pierde
    (Game|SetGamePaused true)
    (Viewport|RemoveAllWidgets)
    (bind _returnvalue_3 (UserInterface|CreateWidget "/Game/Blueprints/BP_Widgets/Widgets/BPW_GameOver.BPW_GameOver_C" (Game|GetPlayerController 0)))
    (UserInterface|Viewport|AddtoPlayerScreen _returnvalue_3)
    (Input|SetInputModeUIOnly _returnvalue _returnvalue_3 "DoNotLock")
    (Variables|/Script/Engine.PlayerController|SetbShowMouseCursor _returnvalue true)
    (Audio|SpawnSound2D "/Game/Blueprints/BP_Guide/Sounds/GameLoseSound.GameLoseSound" 1.0 1.0 0.0 0)
    (else
      ;[1 1 1] Jugador gana
      (bind _asfirst_person_character (Utilities|Casting|CastToFirstPersonCharacter (Game|GetPlayerCharacter 0)))
      (if (>= (Variables|/Game/Blueprints/BP_FirstPerson/FirstPersonCharacter.FirstPersonCharacter_C|GetDeadEnemies _asfirst_person_character) 100)
        (Game|SetGamePaused true)
        (Viewport|RemoveAllWidgets)
        (bind _returnvalue_4 (UserInterface|CreateWidget "/Game/Blueprints/BP_Widgets/Widgets/BPW_PlayerWin.BPW_PlayerWin_C" (Game|GetPlayerController 0)))
        (UserInterface|Viewport|AddtoPlayerScreen _returnvalue_4)
        (Input|SetInputModeUIOnly _returnvalue_2 _returnvalue_4 "DoNotLock")
        (Variables|/Script/Engine.PlayerController|SetbShowMouseCursor _returnvalue_2 true)
        (Audio|SpawnSound2D "/Game/Blueprints/BP_Guide/Sounds/GameWinSound.GameWinSound" 1.0 1.0 0.0 0)))))

(event EventBeginPlay
  (Utilities|StartGame))

(fn ConstructionScript)

(fn MunitionCollected
  (Variables|Default|SetMunition (+ (Variables|Default|GetMunition) 200)))

(fn Shoot
  (Variables|Default|SetMunition (- (Variables|Default|GetMunition) 1)))

(fn Hit
  (Variables|Default|SetHealth (- (Variables|Default|GetHealth) 20)))

(fn SpeedMunitionCollected
  (Variables|Default|SetSuper true))